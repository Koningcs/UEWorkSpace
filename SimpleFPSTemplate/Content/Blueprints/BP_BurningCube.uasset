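; BP_BurningCube is an actor that plays a burn-away dissolve effect on its static mesh and then destroys itself.
; BeginPlay sets initial DissolveAlpha, EdgeLerp and Tiling material parameters, waits briefly, then plays the DissolveTime timeline.
; Each timeline update drives those three parameters, with DissolveAlpha offset from its curve.
; The delayed DestroyActor hangs off the Update pin, so its countdown starts with the first update rather than on timeline completion.
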(event EventBeginPlay
  (Rendering|Material|SetScalarParameterValueonMaterials (Variables|Debug|GetStaticMeshComponent) "DissolveAlpha" (Variables|Default|GetDissolveAlpha))
  (Rendering|Material|SetScalarParameterValueonMaterials (Variables|Debug|GetStaticMeshComponent) "EdgeLerp" (Variables|Default|GetEdgeLerp))
  (Rendering|Material|SetScalarParameterValueonMaterials (Variables|Debug|GetStaticMeshComponent) "Tiling" (Variables|Default|GetTiling))
  (Utilities|FlowControl|Delay 2.0)
  (bind (_direction _dissolvetime _tilingtime _edgelerptime) (Timeline|DissolveTime PlayFromStart)
    (:Update
      (Utilities|FlowControl|Sequence
        (:then_0
          (Rendering|Material|SetScalarParameterValueonMaterials (Variables|Debug|GetStaticMeshComponent) "DissolveAlpha" (- _dissolvetime 1.0)))
        (:then_1
          (Rendering|Material|SetScalarParameterValueonMaterials (Variables|Debug|GetStaticMeshComponent) "Tiling" _tilingtime))
        (:then_2
          (Rendering|Material|SetScalarParameterValueonMaterials (Variables|Debug|GetStaticMeshComponent) "EdgeLerp" _edgelerptime)
          (Utilities|FlowControl|Delay 2.0)
          (Actor|DestroyActor))))))

(event EventTick
  (params (DeltaSeconds :type Float%20%28single-precision%29)))

(fn ConstructionScript)

(fn Dissolve)